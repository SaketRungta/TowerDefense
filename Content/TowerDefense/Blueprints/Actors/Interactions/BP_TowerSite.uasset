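; BP_TowerSite is an interactive tower site actor for a tower defense game that highlights its mesh under the cursor.
; Cursor-over events on TowerSiteMesh raise the material Emissive parameter on hover and clear it on exit.
; Disabled sites ignore both events, and an active site keeps its glow when the cursor leaves.
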(event `self.TowerSiteMesh.OnBeginCursorOver`
  (params (TouchedComponent :type "PrimitiveComponent Object Reference"))
  (if (not (`self.GetIsSiteDisabled`))
    (`MeshComponent.SetScalarParameterValueOnMaterials` (`self.GetTowerSiteMesh`) "Emissive" 2.0)))

(event `self.TowerSiteMesh.OnEndCursorOver`
  (params (TouchedComponent :type "PrimitiveComponent Object Reference"))
  (if (`self.GetIsSiteDisabled`)
    _
    (elif (not (`self.GetIsSiteActive`))
      (`MeshComponent.SetScalarParameterValueOnMaterials` (`self.GetTowerSiteMesh`) "Emissive" 0.0))))

(fn `UserConstructionScript`)