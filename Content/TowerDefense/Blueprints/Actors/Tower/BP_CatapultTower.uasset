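; Catapult tower for the tower defense game that animates the throwing motion and launch of its projectile.
; FireCatapult plays a sped-up timeline that pitches the turret mesh through its swing, then calls FireProjectile when the swing finishes.
; After a short delay, RetreatCatapult eases the mesh back with a second timeline, then unhides the loaded projectile mesh after another pause.
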(event `self.FireCatapult`
  (`TimelineComponent.SetPlayRate` (`self.TL_CatapultFire`) 4.0)
  (bind (_direction _alpha) (`Timeline|TL_CatapultFire` :!via `PlayFromStart`)
    (:`Update`
      (`self.SetTurretMeshPitch` (`KismetMathLibrary.Lerp` 0.0 -80.0 _alpha)))
    (:`Finished`
      (`self.FireProjectile`)
      (`KismetSystemLibrary.Delay` 0.3)
      (`self.RetreatCatapult`))))

(event `RetreatCatapult`
  (bind (_direction _alpha) (`Timeline|TL_CatapultRetreat` :!via `PlayFromStart`)
    (:`Update`
      (`self.SetTurretMeshPitch` (`KismetMathLibrary.Lerp` -80.0 0.0 _alpha)))
    (:`Finished`
      (`KismetSystemLibrary.Delay` 1.0)
      (`SceneComponent.SetHiddenInGame` (`self.GetCatapultProjectileMesh`) false false))))

(fn `UserConstructionScript`)