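; Decor actor for the tower defense game, named as a tree filler quad, that gives itself a random look.
; SetRandomDecor picks a random mesh from DecorMeshes for SMDecor and sets the actor's yaw to a random quarter turn.
; It runs in both the Construction Script and BeginPlay, so the look chosen at construction is rolled again when play begins.
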(event `self.ReceiveBeginPlay`
  (`self.Set Random Decor`))

(fn `Set Random Decor`
  (`StaticMeshComponent.SetStaticMesh` (`self.SM_Decor`) (`|GetArrayItem` (`self.DecorMeshes`) (`KismetMathLibrary.RandomIntegerInRange` 0 (- (`KismetArrayLibrary.Array_Length` (`self.DecorMeshes`)) 1))))
  (`self.K2_SetActorRotation` (`KismetMathLibrary.MakeRotator` 0.0 0.0 (`KismetMathLibrary.Conv_IntToDouble` (* (`KismetMathLibrary.RandomIntegerInRange` 0 3) 90)))))

(fn `UserConstructionScript`
  (`self.Set Random Decor`))