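; Save game object for the tower defense game that holds audio volumes and level progress.
; Audio functions get and set the music and sound volume together.
; SetLevelData works on parallel per-level arrays, keeping the highest star count for a valid level index and unlocking the next level if one exists.
; It also prints the star comparison result as debug output.
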(fn `GetAudioData`
  (returns (MusicVolmue :type "Float (double-precision)") (SoundVolume :type "Float (double-precision)"))
  (return (`self.MusicVolume`) (`self.SoundVolume`)))

(fn `SetAudioData`
  (params (MusicVolume :type "Float (double-precision)") (SoundVolume :type "Float (double-precision)"))
  (set `self.MusicVolume` MusicVolume)
  (set `self.SoundVolume` SoundVolume))

(fn `SetLevelData`
  (params (LevelIndex :type Integer) (StarsCount :type Integer))
  (bind _returnvalue (< (`|GetArrayItem` (`self.LevelStarsCount`) (`local.LevelIndex`)) (`local.StarsCount`)))
  (if (`KismetArrayLibrary.Array_IsValidIndex` (`self.LevelStarsCount`) LevelIndex)
    (`KismetSystemLibrary.PrintString` null (`KismetStringLibrary.Conv_BoolToString` _returnvalue))
    (if _returnvalue
      (`KismetArrayLibrary.Array_Set` (`self.LevelStarsCount`) (`local.LevelIndex`) (`local.StarsCount`)))
    (if (`KismetArrayLibrary.Array_IsValidIndex` (`self.LevelActivatedArray`) (+ (`local.LevelIndex`) 1))
      (`KismetArrayLibrary.Array_Set` (`self.LevelActivatedArray`) (+ (`local.LevelIndex`) 1) true)
      (return))))